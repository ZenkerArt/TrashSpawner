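; Trash scattering tool that drops simulated trash during play and recreates the saved result as static mesh actors.
; While DropTrash is on, Tick uses a Rate-based delay to spawn BP_Simulation_Trash at random points and rotations in a root-scaled box, with random meshes from the TrashPack table.
; EndPlay writes their meshes and transforms to JSON under the project directory.
; LoadLastSimulation reads that file and places StaticMeshActors into a named folder.
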(event Custom|LoadLastSimulation
  (bind _returnvalue (Class|KismetSystemLibrary|GetProjectDirectory))
  (bind _save_path (Variables|Default|GetSave%20Path))
  (bind _array (Utilities|Array|MakeArray _returnvalue _save_path))
  (bind _returnvalue_2 (Utilities|String|JoinStringArray _array "/"))
  (Development|PrintString _returnvalue_2)
  (bind _outjsonobject (Class|JsonBlueprintFunctionLibrary|FromFile (Utilities|Struct|MakeFilePath _returnvalue_2)))
  (bind _outvalue (|GetJsonField _outjsonobject "Test"))
  (bind _output_get (Variables|Default|SetTrashes _outvalue))
  (for _array_element _output_get
    (bind _returnvalue_3 (Game|SpawnActorfromClass "/Script/Engine.StaticMeshActor" (|ZeroPosition) "Undefined" "MultiplyWithRoot" 0 0))
    (Components|StaticMesh|SetStaticMesh (Variables|/Script/Engine.StaticMeshActor|GetStaticMeshComponent _returnvalue_3) (.StaticMesh (Utilities|Struct|BreakF_Trash_Position _array_element)))
    (Class|TrashLib|MoveActortoFolder _returnvalue_3 (Variables|Default|GetFolder%20Name))
    (Transformation|SetActorTransform _returnvalue_3 (.Transforms (Utilities|Struct|BreakF_Trash_Position _array_element)))))

(event EventBeginPlay)

(event EventTick
  (params (DeltaSeconds :type Float%20%28single-precision%29))
  (bind _returnvalue (Math|Random|RandomRotator false))
  (bind _defaultsceneroot (Variables|Default|GetDefaultSceneRoot))
  (bind _defaultsceneroot_2 (Variables|Default|GetDefaultSceneRoot))
  (bind _returnvalue_2 (Transformation|GetWorldLocation _defaultsceneroot_2))
  (bind _returnvalue_3 (Transformation|GetWorldScale _defaultsceneroot))
  (bind _returnvalue_4 (* _returnvalue_3 "50.000000,50.000000,50.000000"))
  (bind _returnvalue_5 (Math|Random|RandomPointinBoundingBox "0, 0, 0" _returnvalue_4))
  (bind _returnvalue_6 (+ _returnvalue_5 _returnvalue_2))
  (bind _returnvalue_7 (Math|Transform|MakeTransform _returnvalue_6 _returnvalue))
  (if (Variables|Default|GetDrop%20Trash)
    (Utilities|FlowControl|Delay (- 1.0 (Variables|Default|GetRate)))
    (bind _returnvalue_8 (Utilities|GetDataTableRow (Variables|Default|GetTrash%20Pack) "Trashes")
      (:then
        (bind _returnvalue_9 (Game|SpawnActorfromClass "/TrashSpawnerPlugin/TrashSpawner/Blueprints/BP_Simulation_Trash.BP_Simulation_Trash_C" _returnvalue_7 "Undefined" "MultiplyWithRoot" 0 0))
        (Components|StaticMesh|SetStaticMesh (Variables|/TrashSpawnerPlugin/TrashSpawner/Blueprints/BP_Simulation_Trash.BP_Simulation_Trash_C|GetCube _returnvalue_9) (.Output (Utilities|GetRandomElement (Utilities|Struct|BreakF_Trash_Pack _returnvalue_8))))
        (Transformation|SetActorTransform _returnvalue_9 _returnvalue_7)
        (Transformation|AddActorWorldOffset _returnvalue_9 "20.000000,0.000000,0.000000")))))

(event EventEndPlay
  (params (EndPlayReason :type EEndPlayReason%20Enum :default "Destroyed"))
  (bind _jsonobjectwrapper (Utilities|Struct|MakeJsonObjectWrapper))
  (Utilities|Array|Clear (Variables|Default|GetTrashes))
  (bind _outactors (Actor|GetAllActorsOfClass "/TrashSpawnerPlugin/TrashSpawner/Blueprints/BP_Simulation_Trash.BP_Simulation_Trash_C"))
  (for _array_element _outactors
    (Utilities|Array|Add (Variables|Default|GetTrashes) (Utilities|Struct|MakeF_Trash_Position (Variables|/Script/Engine.StaticMeshComponent|GetStaticMesh (Variables|/TrashSpawnerPlugin/TrashSpawner/Blueprints/BP_Simulation_Trash.BP_Simulation_Trash_C|GetCube _array_element)) (Transformation|GetWorldTransform (Variables|/TrashSpawnerPlugin/TrashSpawner/Blueprints/BP_Simulation_Trash.BP_Simulation_Trash_C|GetCube _array_element)))))
  (|SetJsonField _jsonobjectwrapper "Test" (Variables|Default|GetTrashes))
  (Class|JsonBlueprintFunctionLibrary|ToFile _jsonobjectwrapper (Utilities|Struct|MakeFilePath (Utilities|String|JoinStringArray (Utilities|Array|MakeArray (Class|KismetSystemLibrary|GetProjectDirectory) (Variables|Default|GetSave%20Path)) "/")))
  (Development|PrintString "Save File"))

(fn ConstructionScript)